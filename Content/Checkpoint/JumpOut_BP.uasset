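; JumpOut_BP is a checkpoint-folder actor that provides three teleport destinations for karts.
; Each of the events TpKart1, TpKart2 and TpKart3 teleports the passed-in target to the world location of its matching numbered component.
; All three events take the destination rotation from a shared Arrow component, so every target faces the same way.
; The Blueprint contains no trigger logic, and its construction script is empty.
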(event `TpKart1`
  (params (NewParam :type "/Game/KartController/BP_KartController Object Reference"))
  (bind _returnvalue_location (`KismetMathLibrary.BreakTransform` (`SceneComponent.K2_GetComponentToWorld` (`self.1`))))
  (`self.K2_TeleportTo` NewParam _returnvalue_location (`SceneComponent.K2_GetComponentRotation` (`self.Arrow`))))

(event `TpKart2`
  (params (NewParam :type "/Game/KartController/BP_KartController Object Reference"))
  (bind _returnvalue_location (`KismetMathLibrary.BreakTransform` (`SceneComponent.K2_GetComponentToWorld` (`self.2`))))
  (`self.K2_TeleportTo` NewParam _returnvalue_location (`SceneComponent.K2_GetComponentRotation` (`self.Arrow`))))

(event `TpKart3`
  (params (NewParam :type "/Game/KartController/BP_KartController Object Reference"))
  (bind _returnvalue_location (`KismetMathLibrary.BreakTransform` (`SceneComponent.K2_GetComponentToWorld` (`self.3`))))
  (`self.K2_TeleportTo` NewParam _returnvalue_location (`SceneComponent.K2_GetComponentRotation` (`self.Arrow`))))

(fn `UserConstructionScript`)