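; JumpIn_BP is a checkpoint-gated jump entrance that hands overlapping karts to a linked JumpOut for teleporting.
; Three trigger components, named 1, 2 and 3, each accept a BP_KartController only if its MLastCheckpoint equals LastPont.
; Triggers 1, 2 and 3 call TpKart3, TpKart2 and TpKart1 respectively, reversing the numbering, then print a debug "Hello".
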(event `self.1.OnComponentBeginOverlap`
  (params (OverlappedComponent :type "PrimitiveComponent Object Reference") (OtherActor :type "Actor Object Reference") (OtherComp :type "PrimitiveComponent Object Reference") (OtherBodyIndex :type Integer) (bFromSweep :type Boolean) (SweepResult :type "HitResult Structure (by ref)"))
  (bind _asbp_kart_controller (cast `/Game/KartController/BP_KartController` OtherActor))
  (if (== (`/Game/KartController/BP_KartController.m_lastCheckpoint` _asbp_kart_controller) (`self.LastPont`))
    (`/Game/Checkpoint/JumpOut_BP.TpKart3` (`self.JumpOut`) _asbp_kart_controller)
    (`KismetSystemLibrary.PrintString` "Hello")))

(event `self.2.OnComponentBeginOverlap`
  (params (OverlappedComponent :type "PrimitiveComponent Object Reference") (OtherActor :type "Actor Object Reference") (OtherComp :type "PrimitiveComponent Object Reference") (OtherBodyIndex :type Integer) (bFromSweep :type Boolean) (SweepResult :type "HitResult Structure (by ref)"))
  (bind _asbp_kart_controller (cast `/Game/KartController/BP_KartController` OtherActor))
  (if (== (`/Game/KartController/BP_KartController.m_lastCheckpoint` _asbp_kart_controller) (`self.LastPont`))
    (`/Game/Checkpoint/JumpOut_BP.TpKart2` (`self.JumpOut`) _asbp_kart_controller)
    (`KismetSystemLibrary.PrintString` "Hello")))

(event `self.3.OnComponentBeginOverlap`
  (params (OverlappedComponent :type "PrimitiveComponent Object Reference") (OtherActor :type "Actor Object Reference") (OtherComp :type "PrimitiveComponent Object Reference") (OtherBodyIndex :type Integer) (bFromSweep :type Boolean) (SweepResult :type "HitResult Structure (by ref)"))
  (bind _asbp_kart_controller (cast `/Game/KartController/BP_KartController` OtherActor))
  (if (== (`/Game/KartController/BP_KartController.m_lastCheckpoint` _asbp_kart_controller) (`self.LastPont`))
    (`/Game/Checkpoint/JumpOut_BP.TpKart1` (`self.JumpOut`) _asbp_kart_controller)
    (`KismetSystemLibrary.PrintString` "Hello")))

(fn `UserConstructionScript`)