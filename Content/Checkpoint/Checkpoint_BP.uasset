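; Race checkpoint actor for a kart game that registers itself in the Mario_GameMode checkpoint array by its MyPoint index.
; Its box overlap advances the kart's last checkpoint to MyPoint + 1.
; Tick measures each PlayersOnMe kart's distance and roughly ranks them for the HUD place display.
; The ranking looks unfinished: the code adding karts to PlayersOnMe is disconnected, as is the new-lap logic.
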(event `self.ReceiveBeginPlay`
  (bind _asmario_game_mode (cast `/Game/Mario_GameMode` (`GameplayStatics.GetGameMode`)))
  (`KismetArrayLibrary.Array_Set` (`/Game/Mario_GameMode.Checkponts` _asmario_game_mode) (`self.MyPoint`) self true))

(event `self.ReceiveTick`
  (params (DeltaSeconds :type "Float (single-precision)"))
  (`KismetArrayLibrary.Array_Clear` (`self.PlayersOnMe_0`))
  (for (_array_element _array_index) (`self.PlayersOnMe`)
    (bind _asbp_kart_controller (cast `/Game/KartController/BP_KartController` _array_element))
    (bind _output_get (set `/Game/KartController/BP_KartController.m_DistensToCheckpont` (`self.GetDistanceTo` _asbp_kart_controller) _asbp_kart_controller))
    (if (== _array_index 0)
      (`KismetArrayLibrary.Array_Set` (`self.PlayersOnMe_0`) 0 (`|GetArrayItem` (`self.PlayersOnMe`)) true)
      (bind _ui_playerplace (`/Game/UI/UI_Widgets/HUD/UI_HUD.UI_PlayerPlace` (`/Game/KartController/BP_KartController.m_UI_HUD` _asbp_kart_controller)))
      (set `/Game/UI/UI_Widgets/HUD/UI_PlayerPlace.Plays` 1 _ui_playerplace)
      (elif (<= (`/Game/KartController/BP_KartController.m_DistensToCheckpont` (`|GetArrayItem` (`self.PlayersOnMe_0`))) _output_get)
        (bind _output_get_2 (set `self.Plays` 0))
        (`self.NewFunction_0` _asbp_kart_controller _ui_playerplace _output_get_2)
        (elif (<= _output_get (`/Game/KartController/BP_KartController.m_DistensToCheckpont` (`|GetArrayItem` (`self.PlayersOnMe_0`) 1)))
          (`self.NewMacro_0` _asbp_kart_controller))))))

(event `self.Box.OnComponentBeginOverlap`
  (params (OverlappedComponent :type "PrimitiveComponent Object Reference") (OtherActor :type "Actor Object Reference") (OtherComp :type "PrimitiveComponent Object Reference") (OtherBodyIndex :type Integer) (bFromSweep :type Boolean) (SweepResult :type "HitResult Structure (by ref)"))
  (bind _asbp_kart_controller (cast `/Game/KartController/BP_KartController` OtherActor))
  (set `/Game/KartController/BP_KartController.m_lastCheckpoint` (+ (`self.MyPoint`) 1) _asbp_kart_controller)
  (`KismetSystemLibrary.PrintString` "NewCheckpont"))

(fn `UserConstructionScript`)