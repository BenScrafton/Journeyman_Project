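; Boost pad that multiplies an overlapping kart's current and max velocity, capped at a scaled default maximum, with optional slow immunity.
; BeginPlay caches default speed, FOV and arm length from the first kart found after a short delay.
; A timeline, offset by boost time, drives max velocity during slowdown and ends immunity.
; Two more timelines widen camera FOV and extend the spring arm, reversing after the boost time.
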(event `self.ReceiveTick`
  (params (DeltaSeconds :type "Float (single-precision)"))
  (bind _as_bp_kart_controller (`self.As BP Kart Controller`))
  ;[1 1 1] Tick
  (if (`self.m_debug`)
    (`KismetSystemLibrary.PrintString` (`KismetStringLibrary.Concat_StrStr` (`KismetStringLibrary.Conv_DoubleToString` (`/Game/KartController/BP_KartController.m_curVelocity` _as_bp_kart_controller)) "/" (`KismetStringLibrary.Conv_DoubleToString` (`/Game/KartController/BP_KartController.m_maxVelocity` _as_bp_kart_controller))))))

(event `self.ReceiveBeginPlay`
  ;[1 1 1] Initialisation
  (`KismetSystemLibrary.Delay` 0.1)
  (bind _outactors (`GameplayStatics.GetAllActorsOfClass` "/Game/KartController/BP_KartController.BP_KartController_C"))
  (bind _output (`|GetArrayItem` _outactors))
  (set `self.As BP Kart Controller` _output)
  (set `self.m_defaultMaxVelocity` (`/Game/KartController/BP_KartController.m_maxVelocity` _output))
  (set `self.m_defaultFOV` (`CameraComponent.FieldOfView` (`/Game/KartController/BP_KartController.Camera` (`self.As BP Kart Controller`))))
  (set `self.m_clampMaxVelocity` (* (`self.m_defaultMaxVelocity`) (`self.m_speedModifier`)))
  (set `self.m_defaultArmLength` (`SpringArmComponent.TargetArmLength` (`/Game/KartController/BP_KartController.SpringArm` (`self.As BP Kart Controller`))))
  (if (`self.m_debug`)
    (`KismetSystemLibrary.PrintString` "Boost Pad Initialisation Complete" true true (struct :`G` 1.0 :`B` 0.046007 :`A` 1.0))))

(event `self.HitBox.OnComponentBeginOverlap`
  (params (OverlappedComponent :type "PrimitiveComponent Object Reference") (OtherActor :type "Actor Object Reference") (OtherComp :type "PrimitiveComponent Object Reference") (OtherBodyIndex :type Integer) (bFromSweep :type Boolean) (SweepResult :type "HitResult Structure (by ref)"))
  (bind _as_bp_kart_controller (`self.As BP Kart Controller`))
  ;[1 1 1] Begin Overlap
  (bind _asbp_kart_controller (cast `/Game/KartController/BP_KartController` OtherActor))
  (bind _output_get (set `self.As BP Kart Controller` _asbp_kart_controller))
  (bind _returnvalue (* (`/Game/KartController/BP_KartController.m_curVelocity` _output_get) (`self.m_speedModifier`)))
  (bind _returnvalue_2 (`KismetMathLibrary.FClamp` _returnvalue 0.0 (`self.m_clampMaxVelocity`)))
  ;;[1 1 1] Adding Speed to Actor
  (set `/Game/KartController/BP_KartController.m_maxVelocity` _returnvalue_2 _as_bp_kart_controller)
  (set `/Game/KartController/BP_KartController.m_curVelocity` _returnvalue_2 _as_bp_kart_controller)
  (set `self.m_additionalVelocity` _returnvalue)
  (`self.IncreaseFOV`)
  (if (`self.m_grantsSlowImmunity?`)
    (set `/Game/KartController/BP_KartController.m_slowImmune` true (`self.As BP Kart Controller`)))
  (`|ExecutionSequence`
    (:`then_0`
      ;;[1 1 1] Slowing Actor Down
      (bind (_direction _multiplier) (`Timeline|SpeedInterp` :`NewTime` (- 10.0 (+ (`self.m_boostTime`) 2.0)) :!via `SetNewTime` :!label _label)
        (:`Update`
          (bind _output_get_2 (set `/Game/KartController/BP_KartController.m_maxVelocity` (+ (* _multiplier (`self.m_additionalVelocity`)) (`self.m_defaultMaxVelocity`)) (`self.As BP Kart Controller`)))
          (if (`self.m_debug`)
            _))
        (:`Finished`
          (if (`self.m_grantsSlowImmunity?`)
            (set `/Game/KartController/BP_KartController.m_slowImmune` false (`self.As BP Kart Controller`))))))
    (:`then_1`
      (goto _label))))

(event `IncreaseFOV`
  ;[1 1 1] IncreaseFOV
  (`|ExecutionSequence`
    (:`then_0`
      (set `self.m_decreasingFOV?` false)
      (if (`self.m_debug`)
        (`KismetSystemLibrary.PrintString` "FOV" true true (struct :`R` 0.923035 :`B` 1.0 :`A` 1.0))
        (bind (_direction _multiplier) (`Timeline|FOVTimelineInit` :!label _label_2) ; IncreasingFOV
          (:`Update`
            (`CameraComponent.SetFieldOfView` (`/Game/KartController/BP_KartController.Camera` (`self.As BP Kart Controller`)) (+ (`self.m_defaultFOV`) (* _multiplier (`self.m_increaseFOV`)))))
          (:`Finished`
            (if (not (`self.m_decreasingFOV?`))
              (set `self.m_decreasingFOV?` true)
              (`KismetSystemLibrary.Delay` (`self.m_boostTime`))
              (if (`self.m_decreasingFOV?`)
                (goto _label_2 :!via `Reverse`)))))
        (else
          (goto _label_2))))
    (:`then_1`
      (`self.ExtendSpringArm`))))

(event `ExtendSpringArm`
  (`KismetSystemLibrary.PrintString` "ARM")
  (set `self.m_decreasingSpring?` false)
  (bind (_direction _multiplier) (`Timeline|Timeline_0` :!label _label_3) ; IncreasingFOV
    (:`Update`
      (set `SpringArmComponent.TargetArmLength` (+ (`self.m_defaultArmLength`) (* _multiplier (`self.m_increaseArm`))) (`/Game/KartController/BP_KartController.SpringArm` (`self.As BP Kart Controller`))))
    (:`Finished`
      (if (not (`self.m_decreasingSpring?`))
        (set `self.m_decreasingSpring?` true)
        (`KismetSystemLibrary.Delay` (`self.m_boostTime`))
        (goto _label_3 :!via `Reverse`)))))

(fn `UserConstructionScript`)