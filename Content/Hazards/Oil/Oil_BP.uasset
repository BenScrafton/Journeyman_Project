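; Oil hazard Blueprint that slows karts that drive into it.
; When HitBox begins overlapping a BP_KartController, it checks the kart's MSlowImmune flag.
; Karts that are not immune lose a fraction of their MCurVelocity set by MSlowModifier, as a one-time cut on each overlap with no timer or restore.
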(event `self.HitBox.OnComponentBeginOverlap`
  (params (OverlappedComponent :type "PrimitiveComponent Object Reference") (OtherActor :type "Actor Object Reference") (OtherComp :type "PrimitiveComponent Object Reference") (OtherBodyIndex :type Integer) (bFromSweep :type Boolean) (SweepResult :type "HitResult Structure (by ref)"))
  (bind _as_bp_kart_controller (`self.As BP Kart Controller`))
  (bind _m_curvelocity (`/Game/KartController/BP_KartController.m_curVelocity` _as_bp_kart_controller))
  (bind _asbp_kart_controller (cast `/Game/KartController/BP_KartController` OtherActor))
  (bind _output_get (set `self.As BP Kart Controller` _asbp_kart_controller))
  (if (not (`/Game/KartController/BP_KartController.m_slowImmune` _output_get))
    ;[1 1 1] Calculates Velocity after Hit
    (set `/Game/KartController/BP_KartController.m_curVelocity` (- _m_curvelocity (* _m_curvelocity (`self.m_slowModifier`))) _as_bp_kart_controller)))

(fn `UserConstructionScript`)