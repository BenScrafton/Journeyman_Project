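; Oil slick hazard that slows karts and makes their handling slippery on contact.
; Shortly after BeginPlay it caches default steer factor and deceleration from the first BP_KartController found in the level.
; When HitBox overlaps a kart without slow immunity, it cuts velocity by a fraction and overrides steering and deceleration.
; After the slippy duration, a Delay restores those cached defaults on the last stored kart reference.
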(event `self.ReceiveBeginPlay`
  ;[1 1 1] Initialisation
  (`KismetSystemLibrary.Delay` 0.1)
  (bind _outactors (`GameplayStatics.GetAllActorsOfClass` "/Game/KartController/BP_KartController.BP_KartController_C"))
  (bind _output_get (set `self.As BP Kart Controller` (`|GetArrayItem` _outactors)))
  (set `self.m_defaultSteerFactor` (`/Game/KartController/BP_KartController.m_steerFactor` _output_get))
  (set `self.m_defaultDeceleration` (`/Game/KartController/BP_KartController.m_deceleration` _output_get)))

(event `self.HitBox.OnComponentBeginOverlap`
  (params (OverlappedComponent :type "PrimitiveComponent Object Reference") (OtherActor :type "Actor Object Reference") (OtherComp :type "PrimitiveComponent Object Reference") (OtherBodyIndex :type Integer) (bFromSweep :type Boolean) (SweepResult :type "HitResult Structure (by ref)"))
  (bind _as_bp_kart_controller (`self.As BP Kart Controller`))
  (bind _as_bp_kart_controller_2 (`self.As BP Kart Controller`))
  (bind _as_bp_kart_controller_3 (`self.As BP Kart Controller`))
  (bind _m_curvelocity (`/Game/KartController/BP_KartController.m_curVelocity` _as_bp_kart_controller))
  ;[1 1 1] Begin Ovelap
  (bind _asbp_kart_controller (cast `/Game/KartController/BP_KartController` OtherActor))
  (bind _output_get (set `self.As BP Kart Controller` _asbp_kart_controller))
  (if (not (`/Game/KartController/BP_KartController.m_slowImmune` _output_get))
    ;;[1 1 1] Calculates Velocity after Hit
    (set `/Game/KartController/BP_KartController.m_curVelocity` (- _m_curvelocity (* _m_curvelocity (`self.m_slowModifier`))) _as_bp_kart_controller)
    ;;[1 1 1] Slippy Controls
    (set `/Game/KartController/BP_KartController.m_steerFactor` (`self.m_newSteerFactor`) _as_bp_kart_controller_2)
    (set `/Game/KartController/BP_KartController.m_deceleration` (`self.m_newDeceleration`) _as_bp_kart_controller_2)
    (`KismetSystemLibrary.Delay` (`self.m_slippyDuration`))
    (set `/Game/KartController/BP_KartController.m_steerFactor` (`self.m_defaultSteerFactor`) _as_bp_kart_controller_3)
    (set `/Game/KartController/BP_KartController.m_deceleration` (`self.m_defaultDeceleration`) _as_bp_kart_controller_3)))

(fn `UserConstructionScript`)