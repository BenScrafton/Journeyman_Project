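; Destructible cactus hazard that slows a kart on overlap, playing a hit particle and sound and removing its mesh and hitbox.
; Current speed decides the penalty: fast or stationary, non-accelerating karts get reduced max velocity, while slow-moving ones only lose current velocity.
; After a delay it restores the max velocity cached at BeginPlay from the first kart found, then destroys itself.
; Non-moving but accelerating karts skip both penalty and actor destruction.
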(event `self.ReceiveBeginPlay`
  ;[1 1 1] Initialisation
  (bind _returnvalue (`GameplayStatics.GetActorOfClass` "/Game/KartController/BP_KartController.BP_KartController_C"))
  (set `self.DefaultMaxVelocity` (`/Game/KartController/BP_KartController.m_maxVelocity` _returnvalue)))

(event `self.HitBox.OnComponentBeginOverlap`
  (params (OverlappedComponent :type "PrimitiveComponent Object Reference") (OtherActor :type "Actor Object Reference") (OtherComp :type "PrimitiveComponent Object Reference") (OtherBodyIndex :type Integer) (bFromSweep :type Boolean) (SweepResult :type "HitResult Structure (by ref)"))
  ;[1 1 1] Overlap
  (bind _asbp_kart_controller (cast `/Game/KartController/BP_KartController` OtherActor))
  (`self.Spawn Effects`)
  (`self.RemoveMesh/HitboxComponents`)
  (set `self.PlayerREF` _asbp_kart_controller)
  (bind _m_curvelocity (`/Game/KartController/BP_KartController.m_curVelocity` _asbp_kart_controller))
  (if (<= _m_curvelocity 0.0)
    (if (not (`/Game/KartController/BP_KartController.m_isAccelerating` _asbp_kart_controller))
      (set `/Game/KartController/BP_KartController.m_curVelocity` 0.0 _asbp_kart_controller)
      (set `/Game/KartController/BP_KartController.m_maxVelocity` (- (`/Game/KartController/BP_KartController.m_maxVelocity` _asbp_kart_controller) (`self.m_MaxVelocitySlowReduction`)) _asbp_kart_controller :!label _label)
      (`KismetSystemLibrary.Delay` (`self.m_SlowDuration`) :!label _label_2)
      (set `/Game/KartController/BP_KartController.m_maxVelocity` (`self.DefaultMaxVelocity`) (`self.PlayerREF`))
      (`self.K2_DestroyActor`))
    (elif (>= _m_curvelocity 15.0)
      (set `/Game/KartController/BP_KartController.m_curVelocity` (- _m_curvelocity (`self.m_InstantVelocitySlowReduction`)) _asbp_kart_controller)
      (goto _label)
      (else
        (set `/Game/KartController/BP_KartController.m_curVelocity` (- _m_curvelocity (- (`self.m_InstantVelocitySlowReduction`) 5.0)) _asbp_kart_controller)
        (goto _label_2)))))

(event `Spawn Effects`
  (`GameplayStatics.SpawnEmitterAtLocation` "/Game/Particles/P_CactusHit.P_CactusHit" (`SceneComponent.K2_GetComponentLocation` (`self.CactusMesh`)))
  (`GameplayStatics.PlaySoundAtLocation` null (`SceneComponent.K2_GetComponentLocation` (`self.CactusMesh`)) (struct) 1.0 1.0 0.0 null null null))

(event `RemoveMesh/HitboxComponents`
  (bind _cactusmesh (`self.CactusMesh`))
  (`ActorComponent.K2_DestroyComponent` _cactusmesh)
  (`ActorComponent.K2_DestroyComponent` (`self.HitBox`))
  (`PrimitiveComponent.SetCollisionEnabled` _cactusmesh "NoCollision")
  (`PrimitiveComponent.SetCollisionEnabled` (`self.HitBox`) "NoCollision"))

(fn `UserConstructionScript`)