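; BP_PokeyCactus is a cactus hazard meant to move along a BP_PokeySpline and crash karts, but most of its logic is disconnected.
; BeginPlay, overlap, MovePokey and ReversePokey events are empty.
; Unwired chains hold the actor lookups, timeline-driven spline movement with a FlipFlop for direction, and kart crash with delayed sound reset.
; Only PlaySound is wired, playing a hit sound at the mesh through a DoOnce.
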(event `self.ReceiveBeginPlay`)

(event `self.HitBox.OnComponentBeginOverlap`
  (params (OverlappedComponent :type "PrimitiveComponent Object Reference") (OtherActor :type "Actor Object Reference") (OtherComp :type "PrimitiveComponent Object Reference") (OtherBodyIndex :type Integer) (bFromSweep :type Boolean) (SweepResult :type "HitResult Structure (by ref)")))

(event `PlaySound`
  (`/Engine/EditorBlueprintResources/StandardMacros.DoOnce` false
    (:`Completed`
      (`GameplayStatics.PlaySoundAtLocation` "/Game/Audio/CactusImpact/Cactus_hit_sound2.Cactus_hit_sound2" (`SceneComponent.K2_GetComponentLocation` (`self.PokeyCactus_SM`)) (struct) 1.0 1.0 0.0 null null null))))

(event `MovePokey`)

(event `ReversePokey`)

(fn `UserConstructionScript`)