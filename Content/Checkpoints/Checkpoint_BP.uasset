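; Checkpoint trigger actor for a kart race that tracks each kart's progress in order and detects new laps.
; When its Box is overlapped, it advances the kart controller's MLastCheckpoint only if the kart last passed the preceding point.
; Otherwise, a kart already at LastPoint resets to zero and a "New Lap" debug message prints.
; The instance flagged Start copies LastPoint to Mario_GameMode on BeginPlay.
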(event `self.ReceiveBeginPlay`
  (if (`self.Start`)
    (bind _asmario_game_mode (cast `/Game/Mario_GameMode` (`GameplayStatics.GetGameMode`)))
    (set `/Game/Mario_GameMode.LastCheckpont` (`self.LastPoint`) _asmario_game_mode)))

(event `self.Box.OnComponentBeginOverlap`
  (params (OverlappedComponent :type "PrimitiveComponent Object Reference") (OtherActor :type "Actor Object Reference") (OtherComp :type "PrimitiveComponent Object Reference") (OtherBodyIndex :type Integer) (bFromSweep :type Boolean) (SweepResult :type "HitResult Structure (by ref)"))
  (bind _asbp_kart_controller (cast `/Game/KartController/BP_KartController` OtherActor))
  (bind _m_lastcheckpoint (`/Game/KartController/BP_KartController.m_lastCheckpoint` _asbp_kart_controller))
  (if (== _m_lastcheckpoint (- (`self.MyPoint`) 1))
    (set `/Game/KartController/BP_KartController.m_lastCheckpoint` (+ (`/Game/KartController/BP_KartController.m_lastCheckpoint` _asbp_kart_controller) 1) _asbp_kart_controller)
    (`KismetSystemLibrary.PrintString` "NewCheckpont")
    (elif (== _m_lastcheckpoint (`self.LastPoint`))
      (`KismetSystemLibrary.PrintString` "New Lap" true true (struct :`R` 1.0 :`G` 0.046659 :`A` 1.0))
      (set `/Game/KartController/BP_KartController.m_lastCheckpoint` 0 _asbp_kart_controller))))

(fn `UserConstructionScript`)