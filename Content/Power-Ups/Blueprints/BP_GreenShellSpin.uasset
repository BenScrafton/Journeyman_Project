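; Green shell spin power-up actor made of four pairs of sphere components, each pair removed independently on contact.
; Each event destroys both spheres of its pair, leaving the other pairs intact.
; Triggers differ per pair: the first reacts to a hit or begin overlap, the second to begin overlap, and the last two to end overlap.
; The graph holds no spin, damage or spawning logic.
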(event `self.Sphere.OnComponentHit`
  (params (HitComponent :type "PrimitiveComponent Object Reference") (OtherActor :type "Actor Object Reference") (OtherComp :type "PrimitiveComponent Object Reference") (NormalImpulse :type "Vector Structure") (Hit :type "HitResult Structure (by ref)"))
  (`ActorComponent.K2_DestroyComponent` (`self.Sphere`) :!label _label)
  (`ActorComponent.K2_DestroyComponent` (`self.Sphere4`)))

(event `self.Sphere4.OnComponentBeginOverlap`
  (params (OverlappedComponent :type "PrimitiveComponent Object Reference") (OtherActor :type "Actor Object Reference") (OtherComp :type "PrimitiveComponent Object Reference") (OtherBodyIndex :type Integer) (bFromSweep :type Boolean) (SweepResult :type "HitResult Structure (by ref)"))
  (goto _label))

(event `self.Sphere5.OnComponentBeginOverlap`
  (params (OverlappedComponent :type "PrimitiveComponent Object Reference") (OtherActor :type "Actor Object Reference") (OtherComp :type "PrimitiveComponent Object Reference") (OtherBodyIndex :type Integer) (bFromSweep :type Boolean) (SweepResult :type "HitResult Structure (by ref)"))
  (`ActorComponent.K2_DestroyComponent` (`self.Sphere1`))
  (`ActorComponent.K2_DestroyComponent` (`self.Sphere5`)))

(event `self.Sphere6.OnComponentEndOverlap`
  (params (OverlappedComponent :type "PrimitiveComponent Object Reference") (OtherActor :type "Actor Object Reference") (OtherComp :type "PrimitiveComponent Object Reference") (OtherBodyIndex :type Integer))
  (`ActorComponent.K2_DestroyComponent` (`self.Sphere2`))
  (`ActorComponent.K2_DestroyComponent` (`self.Sphere6`)))

(event `self.Sphere7.OnComponentEndOverlap`
  (params (OverlappedComponent :type "PrimitiveComponent Object Reference") (OtherActor :type "Actor Object Reference") (OtherComp :type "PrimitiveComponent Object Reference") (OtherBodyIndex :type Integer))
  (`ActorComponent.K2_DestroyComponent` (`self.Sphere7`))
  (`ActorComponent.K2_DestroyComponent` (`self.Sphere3`)))

(fn `UserConstructionScript`)