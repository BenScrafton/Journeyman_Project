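; BP_FakeBoxPU is the fake box power-up, which places a fake box from the kart that uses it.
; On BeginPlay it spawns a BP_FakeBox at the world transform of MKart's ThrowingLocation, then calls PowerUpUsed on MKart.
; All logic runs in that one event, with overlap and tick left as disabled stubs.
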(event `self.ReceiveBeginPlay`
  (bind _m_kart (`self.m_kart`))
  (`parent.ReceiveBeginPlay`)
  (`|SpawnActorFromClass` "/Game/Power-Ups/Blueprints/BP_FakeBox.BP_FakeBox_C" (`SceneComponent.K2_GetComponentToWorld` (`/Game/KartController/BP_KartController.ThrowingLocation` _m_kart)) "Undefined" "OverrideRootScale" null null)
  (`/Game/KartController/BP_KartController.PowerUpUsed` _m_kart))

(fn `UserConstructionScript`
  (`parent.UserConstructionScript`))