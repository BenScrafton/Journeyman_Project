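; BP_OrientComp is a component that tilts its owning actor to match the surface beneath it.
; Each tick it runs a Visibility line trace from the owner along its local down axis.
; On a hit, it derives roll and pitch from the impact normal, keeps the current yaw, and smoothly interpolates the owner's rotation toward that target with RInterpTo.
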(event `self.ReceiveTick`
  (params (DeltaSeconds :type "Float (single-precision)"))
  (bind _returnvalue (`self.GetOwner`))
  (bind _returnvalue_2 (`self.GetOwner`))
  (bind _returnvalue_3 (`Actor.K2_GetActorLocation` _returnvalue_2))
  (bind _returnvalue_4 (`Actor.K2_GetActorRotation` _returnvalue))
  (bind (_outhit _returnvalue_5) (`KismetSystemLibrary.LineTraceSingle` _returnvalue_3 (+ (* (`Actor.GetActorUpVector` _returnvalue_2) -1000) _returnvalue_3) "TraceTypeQuery1"))
  (if _returnvalue_5
    (bind (_bblockinghit _binitialoverlap _time _distance _location _impactpoint _normal _impactnormal) (`GameplayStatics.BreakHitResult` _outhit))
    (`Actor.K2_SetActorRotation` _returnvalue (`KismetMathLibrary.RInterpTo` _returnvalue_4 (`KismetMathLibrary.MakeRotator` (.roll (`KismetMathLibrary.MakeRotFromXZ` (`Actor.GetActorForwardVector` _returnvalue) _impactnormal)) (.pitch (`KismetMathLibrary.MakeRotFromYZ` (`Actor.GetActorRightVector` _returnvalue) _impactnormal)) (.yaw _returnvalue_4)) (`GameplayStatics.GetWorldDeltaSeconds`) 10.0) false)))