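; BP_FireFlowerPU is the Fire Flower kart power-up, a child Blueprint that overrides the inherited UsePowerUp function.
; Each use calls the parent, spawns a BP_FireFlower actor at the kart's ThrowingLocation, increments the use counter and prints a debug count.
; When the counter equals the maximum uses, it calls PowerUpUsed on the kart.
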(event `self.ReceiveBeginPlay`
  (`parent.ReceiveBeginPlay`))

(fn `UsePowerUp`
  (bind _m_kart (`self.m_kart`))
  (bind _returnvalue (+ (`self.m_uses`) 1))
  (`parent.UsePowerUp`)
  (`|SpawnActorFromClass` "/Game/Power-Ups/Blueprints/BP_FireFlower.BP_FireFlower_C" (`SceneComponent.K2_GetComponentToWorld` (`/Game/KartController/BP_KartController.ThrowingLocation` _m_kart)) "Undefined" "OverrideRootScale" null null)
  (set `self.m_uses` _returnvalue)
  (`KismetSystemLibrary.PrintString` (`KismetStringLibrary.Conv_IntToString` _returnvalue))
  (if (== (`self.m_uses`) (`self.m_maxUses`))
    (`/Game/KartController/BP_KartController.PowerUpUsed` _m_kart)))

(fn `UserConstructionScript`
  (`parent.UserConstructionScript`))