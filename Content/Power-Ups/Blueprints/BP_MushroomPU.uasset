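; BP_MushroomPU is the mushroom power-up for a kart racer, built as a child of a parent power-up class.
; Its UsePowerUp override calls the parent, spawns a BP_Mushroom actor at the world origin and passes it the MKart reference.
; It then tells that kart the power-up was used, leaving any effect to the spawned actor.
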(fn `UsePowerUp`
  (bind _m_kart (`self.m_kart`))
  (`parent.UsePowerUp`)
  (bind _returnvalue (`|SpawnActorFromClass` "/Game/Power-Ups/Blueprints/BP_Mushroom.BP_Mushroom_C" (`KismetMathLibrary.MakeTransform` (0.0 0.0 0.0)) "Undefined" "OverrideRootScale" null null))
  (set `/Game/Power-Ups/Blueprints/BP_Mushroom.m_kart` _m_kart _returnvalue)
  (`/Game/KartController/BP_KartController.PowerUpUsed` _m_kart))

(fn `UserConstructionScript`
  (`parent.UserConstructionScript`))