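; BP_Mushroom is a power-up that gives a small speed increase to the kart it references through MKart.
; On BeginPlay it increments the kart's MCurVelocity once, capped at MMaxVelocity, and does nothing if the kart is already at that maximum.
; The file never assigns MKart, and a player-pawn cast to BP_KartController is left unconnected.
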(event `self.ReceiveBeginPlay`
  (bind _m_kart (`self.m_kart`))
  (bind _m_curvelocity (`/Game/KartController/BP_KartController.m_curVelocity` _m_kart))
  (bind _m_maxvelocity (`/Game/KartController/BP_KartController.m_maxVelocity` _m_kart))
  (if (not (== _m_curvelocity _m_maxvelocity))
    (bind _result (`/Engine/EditorBlueprintResources/StandardMacros.IncrementFloat` _m_curvelocity)
      (:`  `
        (if (> _result _m_maxvelocity)
          (set `/Game/KartController/BP_KartController.m_curVelocity` (`/Game/KartController/BP_KartController.m_maxVelocity` _m_kart) _m_kart)
          (else
            (set `/Game/KartController/BP_KartController.m_curVelocity` _result _m_kart)))))))

(fn `UserConstructionScript`)