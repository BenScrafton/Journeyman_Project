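; Kart power-up that puts the owning kart into Bullet Bill mode for a limited time.
; UsePowerUp spawns a BP_BulletBill at the kart's transform, hands it to the kart and sets the active flags.
; While active, Tick runs a Delay of MActiveTime, then clears the kart's flag, calls PowerUpUsed and destroys both the bill and itself.
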(event `self.ReceiveTick`
  (params (DeltaSeconds :type "Float (single-precision)"))
  (bind _m_kart (`self.m_kart`))
  (`parent.ReceiveTick` DeltaSeconds)
  (if (`self.m_isActive`)
    (`KismetSystemLibrary.Delay` (`self.m_activeTime`))
    (set `/Game/KartController/BP_KartController.m_isBulletBill` false _m_kart)
    (`/Game/KartController/BP_KartController.PowerUpUsed` _m_kart)
    (`self.K2_DestroyActor` (`self.m_billRef`))
    (`self.K2_DestroyActor`)))

(fn `UsePowerUp`
  (bind _m_kart (`self.m_kart`))
  (`parent.UsePowerUp`)
  (`KismetSystemLibrary.PrintString` "Hello")
  (bind _returnvalue (`|SpawnActorFromClass` "/Game/Power-Ups/Blueprints/Bill/BP_BulletBill.BP_BulletBill_C" (`self.GetTransform` (`self.m_kart`)) "Undefined" "OverrideRootScale" null null))
  (set `/Game/KartController/BP_KartController.m_isBulletBill` true _m_kart)
  (set `/Game/KartController/BP_KartController.m_bill` _returnvalue _m_kart)
  (set `self.m_isActive` true)
  (set `self.m_billRef` _returnvalue))

(fn `UserConstructionScript`
  (`parent.UserConstructionScript`))