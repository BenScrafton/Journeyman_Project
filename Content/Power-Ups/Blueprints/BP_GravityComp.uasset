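; BP_GravityComp is a component in the Power-Ups folder that applies simple custom gravity to its owner actor.
; Each tick, a debug-drawn line trace along the owner's down vector checks for ground.
; When airborne, it accumulates fall velocity and offsets the owner down world Z; when grounded, it zeroes velocity and lifts the owner to trace length.
; A damped Bounce function with a cutoff exists but is never run.
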(event `self.ReceiveTick`
  (params (DeltaSeconds :type "Float (single-precision)"))
  (bind _m_tracelength (`self.m_traceLength`))
  (bind (_returnvalue _distance) (`self.CheckGrounded`))
  (if _returnvalue
    (set `self.m_curVelocity` 0.0)
    (if (< _distance _m_tracelength)
      (`Actor.K2_AddActorWorldOffset` (`self.GetOwner`) (* (`Actor.GetActorUpVector` (`self.GetOwner`)) (- _m_tracelength _distance)) false false))
    (else
      (set `self.m_curVelocity` (+ (`self.m_curVelocity`) (* (`self.m_strength`) (`GameplayStatics.GetWorldDeltaSeconds`))))
      (`Actor.K2_AddActorWorldOffset` (`self.GetOwner`) (`KismetMathLibrary.MakeVector` 0.0 0.0 (* (`self.m_curVelocity`) (`GameplayStatics.GetWorldDeltaSeconds`) -1.0)) false false))))

(fn `Bounce`
  (if (`self.m_canBounce`)
    (if (<= (`self.m_curVelocity`) (`self.m_bounceCutOff`))
      (set `self.m_curVelocity` 0.0 :!label _label)
      (else
        (if (> (`self.m_curVelocity`) 0.0)
          (set `self.m_curVelocity` (* (`self.m_curVelocity`) -1.0)))
        (set `self.m_curVelocity` (* (`self.m_curVelocity`) (`self.m_bounceFactor`)))))
    (else
      (goto _label))))

(fn `CheckGrounded`
  (returns (ReturnValue :type Boolean) (Distance :type "Float (double-precision)"))
  (bind _returnvalue (`self.GetOwner`))
  (bind _returnvalue_2 (`Actor.K2_GetActorLocation` _returnvalue))
  (bind (_outhit _returnvalue_3) (`KismetSystemLibrary.LineTraceSingle` :`Start` _returnvalue_2 :`End` (+ _returnvalue_2 (* (`Actor.GetActorUpVector` _returnvalue) (* -1 (`self.m_traceLength`)))) :`TraceChannel` "TraceTypeQuery1" :`DrawDebugType` "ForOneFrame" :`TraceColor` (struct :`R` 0.094925 :`G` 1.0 :`A` 1.0)))
  (return _returnvalue_3 (`.Distance` (`GameplayStatics.BreakHitResult` _outhit))))