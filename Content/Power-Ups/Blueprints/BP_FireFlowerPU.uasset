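; Fire Flower power-up for the kart game, which launches a fire flower from the owning kart when used.
; UsePowerUp calls the parent implementation, casts the owner to BP_KartController and stores it as MKart.
; It then spawns a BP_FireFlower at the kart's ThrowingLocation transform and prints a "Hello" debug string.
; The event graph holds only disabled default events.
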(fn `UsePowerUp`
  (`parent.UsePowerUp`)
  (bind _asbp_kart_controller (cast `/Game/KartController/BP_KartController` (`self.GetOwner`)))
  (bind _output_get (set `self.m_kart` _asbp_kart_controller))
  (`|SpawnActorFromClass` "/Game/Power-Ups/Blueprints/BP_FireFlower.BP_FireFlower_C" (`SceneComponent.K2_GetComponentToWorld` (`/Game/KartController/BP_KartController.ThrowingLocation` _output_get)) "Undefined" "OverrideRootScale" null null)
  (`KismetSystemLibrary.PrintString` "Hello"))

(fn `UserConstructionScript`
  (`parent.UserConstructionScript`))