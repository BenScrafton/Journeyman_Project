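; BP_FakeBox is a fake item box power-up that crashes any kart overlapping its mesh.
; Each Tick it traces down along its up vector and moves along its forward vector until the trace distance drops below a small threshold.
; Below that threshold it stops moving and plays a timeline that drives the mesh's relative rotation on all three axes.
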(event `self.ReceiveTick`
  (params (DeltaSeconds :type "Float (single-precision)"))
  (bind _outhit (`KismetSystemLibrary.LineTraceSingle` (`self.K2_GetActorLocation`) (+ (`self.K2_GetActorLocation`) (* (`self.GetActorUpVector`) -1000.0)) "TraceTypeQuery1"))
  (if (< (`.Distance` (`GameplayStatics.BreakHitResult` _outhit)) 4.0)
    (bind (_direction _rotation) (`Timeline|Timeline_0`)
      (:`Update`
        (`SceneComponent.K2_SetRelativeRotation` (`self.StaticMesh`) (`KismetMathLibrary.MakeRotator` _rotation _rotation _rotation) false false)))
    (else
      (`self.K2_AddActorWorldOffset` (* (`self.GetActorForwardVector`) (* (`GameplayStatics.GetWorldDeltaSeconds`) 1000.0))))))

(event `self.StaticMesh.OnComponentBeginOverlap`
  (params (OverlappedComponent :type "PrimitiveComponent Object Reference") (OtherActor :type "Actor Object Reference") (OtherComp :type "PrimitiveComponent Object Reference") (OtherBodyIndex :type Integer) (bFromSweep :type Boolean) (SweepResult :type "HitResult Structure (by ref)"))
  (bind _asbp_kart_controller (cast `/Game/KartController/BP_KartController` OtherActor))
  (`/Game/KartController/BP_KartController.Crash` _asbp_kart_controller))

(fn `UserConstructionScript`)