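; BP_FireFlower is a kart power-up projectile that crashes any BP_KartController its mesh overlaps.
; Tick moves it along its forward vector at MSpeed without sweeping.
; A debug-drawn Visibility trace along the mesh's up vector resets the gravity component's velocity to a fixed value on a hit, apparently to bounce it.
; It does not destroy itself on impact.
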(event `self.ReceiveTick`
  (params (DeltaSeconds :type "Float (single-precision)"))
  (bind _staticmesh (`self.StaticMesh`))
  (bind _returnvalue (`SceneComponent.K2_GetComponentLocation` _staticmesh))
  (`self.K2_AddActorWorldOffset` (* (`self.GetActorForwardVector`) (* (`self.m_speed`) (`GameplayStatics.GetWorldDeltaSeconds`))))
  (bind (_outhit _returnvalue_2) (`KismetSystemLibrary.LineTraceSingle` :`Start` _returnvalue :`End` (+ _returnvalue (* (`SceneComponent.GetUpVector` _staticmesh) (`self.m_traceLength`))) :`TraceChannel` "TraceTypeQuery1" :`DrawDebugType` "ForOneFrame"))
  (if _returnvalue_2
    (set `/Game/Power-Ups/Blueprints/Components/BP_GravityComp.m_curVelocity` -600.0 (`self.BP_GravityComp`))))

(event `self.StaticMesh.OnComponentBeginOverlap`
  (params (OverlappedComponent :type "PrimitiveComponent Object Reference") (OtherActor :type "Actor Object Reference") (OtherComp :type "PrimitiveComponent Object Reference") (OtherBodyIndex :type Integer) (bFromSweep :type Boolean) (SweepResult :type "HitResult Structure (by ref)"))
  (bind _asbp_kart_controller (cast `/Game/KartController/BP_KartController` OtherActor))
  (`/Game/KartController/BP_KartController.Crash` _asbp_kart_controller))

(fn `UserConstructionScript`)