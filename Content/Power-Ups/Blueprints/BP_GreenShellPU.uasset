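; Green shell power-up Blueprint that lets a kart launch a green shell.
; Its UsePowerUp override runs the parent logic, spawns GreenShell_bp at the kart's ThrowingLocation transform, then notifies the kart through PowerUpUsed.
; The event graph holds only disabled default events, so all behavior beyond the inherited logic lives in that override.
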(fn `UsePowerUp`
  (`parent.UsePowerUp`)
  (`|SpawnActorFromClass` "/Game/Power-Ups/Blueprints/GreenShell_bp.GreenShell_bp_C" (`SceneComponent.K2_GetComponentToWorld` (`/Game/KartController/BP_KartController.ThrowingLocation` (`self.m_kart`))) "Undefined" "OverrideRootScale" null null)
  (`/Game/KartController/BP_KartController.PowerUpUsed` (`self.m_kart`)))

(fn `UserConstructionScript`
  (`parent.UserConstructionScript`))