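; Bullet Bill power-up actor that flies along the points of the level's TestSpline, looping back to the first after the last.
; On BeginPlay it finds the spline actor and selects the nearest point as its first target.
; Each Tick it lerps the mesh rotation toward the target point and moves along the actor's forward vector.
; It advances to the next point once within a small distance, restarting the rotation blend.
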(event `self.ReceiveBeginPlay`
  (bind _returnvalue (`GameplayStatics.GetActorOfClass` "/Game/Power-Ups/Blueprints/Bill/testSpline.testSpline_C"))
  (set `self.splineRef` _returnvalue)
  (`self.FindClosestPoint`)
  (set `self.startRot` (`SceneComponent.K2_GetComponentRotation` (`self.StaticMesh`))))

(event `self.ReceiveTick`
  (params (DeltaSeconds :type "Float (single-precision)"))
  (if (< (`KismetMathLibrary.Vector_Distance` (`SplineComponent.GetLocationAtSplinePoint` (`/Game/Power-Ups/Blueprints/Bill/testSpline.Spline` (`self.splineRef`)) (`self.closestPointIndex`) "World") (`self.K2_GetActorLocation`)) 100.0)
    (bind _output_get (set `self.closestPointIndex` (+ (`self.closestPointIndex`) 1)))
    (if (> _output_get (- (`SplineComponent.GetNumberOfSplinePoints` (`/Game/Power-Ups/Blueprints/Bill/testSpline.Spline` (`self.splineRef`))) 1))
      (set `self.closestPointIndex` 0))
    (set `self.startRot` (`SceneComponent.K2_GetComponentRotation` (`self.StaticMesh`)))
    (set `self.alpha` 0.0)
    (else
      (bind _output_get_2 (set `self.alpha` (+ (`self.alpha`) (* (`GameplayStatics.GetWorldDeltaSeconds`) (`self.rot speed`)))))
      (if (> _output_get_2 1.0)
        (set `self.alpha` 1.0))
      (`SceneComponent.K2_SetWorldRotation` (`self.StaticMesh`) (`KismetMathLibrary.RLerp` (`self.startRot`) (`KismetMathLibrary.FindLookAtRotation` (`SceneComponent.K2_GetComponentLocation` (`self.StaticMesh`)) (`SplineComponent.GetLocationAtSplinePoint` (`/Game/Power-Ups/Blueprints/Bill/testSpline.Spline` (`self.splineRef`)) (`self.closestPointIndex`) "World")) (`self.alpha`)) false false)
      (`self.K2_AddActorWorldOffset` (* (`self.GetActorForwardVector`) (* (`self.speed`) (`GameplayStatics.GetWorldDeltaSeconds`)))))))

(event `MoveObject`)

(fn `FindClosestPoint`
  (bind _spline (`/Game/Power-Ups/Blueprints/Bill/testSpline.Spline` (`self.splineRef`)))
  (for _index (range (`SplineComponent.GetNumberOfSplinePoints` _spline))
    (bind _returnvalue (`KismetMathLibrary.Vector_Distance` (`SplineComponent.GetLocationAtSplinePoint` _spline _index "World") (`self.K2_GetActorLocation`)))
    (if (< _returnvalue (`self.bestDist`))
      (set `self.bestDist` _returnvalue)
      (set `self.closestPointIndex` _index))))

(fn `UserConstructionScript`)