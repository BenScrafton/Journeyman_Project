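; Banana power-up hazard that crashes any kart that runs into it.
; While its gravity component reports it is airborne, Tick pushes it forward at constant speed without sweep, stopping once grounded.
; Box overlap with a BP_KartController calls Crash and destroys the banana, first notifying the kart via PowerUpUsed if the owner is a BP_BananaPU.
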(event `self.ReceiveTick`
  (params (DeltaSeconds :type "Float (single-precision)"))
  (bind _returnvalue (`/Game/Power-Ups/Blueprints/Components/BP_GravityComp.CheckGrounded` (`self.BP_GravityComp`)))
  (if (not _returnvalue)
    (`self.K2_AddActorWorldOffset` (* (`self.GetActorForwardVector`) (* (`GameplayStatics.GetWorldDeltaSeconds`) 1000.0)))))

(event `self.Box.OnComponentBeginOverlap`
  (params (OverlappedComponent :type "PrimitiveComponent Object Reference") (OtherActor :type "Actor Object Reference") (OtherComp :type "PrimitiveComponent Object Reference") (OtherBodyIndex :type Integer) (bFromSweep :type Boolean) (SweepResult :type "HitResult Structure (by ref)"))
  (bind _asbp_kart_controller (cast `/Game/KartController/BP_KartController` OtherActor))
  (`/Game/KartController/BP_KartController.Crash` _asbp_kart_controller)
  (bind _asbp_banana_pu (cast `/Game/Power-Ups/Blueprints/BP_BananaPU` (`self.GetOwner`))
    (:`then`
      (`/Game/KartController/BP_KartController.PowerUpUsed` (`/Game/Power-Ups/Blueprints/BP_PowerUpBase.m_kart` _asbp_banana_pu))
      (`self.K2_DestroyActor`)
      (`KismetSystemLibrary.PrintString` "Hello"))
    (:`CastFailed`
      (`self.K2_DestroyActor`))))

(fn `UserConstructionScript`)