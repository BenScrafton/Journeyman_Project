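; Kart power-up pickup block with spinning meshes, optionally doubled, that fills a kart's empty primary and secondary power-up slots.
; Overlap rolls random power-ups from an enum array, writing to the first kart controller cached at BeginPlay.
; Taken blocks disable collision, shrink by timeline and return after a delay.
; A double block hit with primary filled shrinks only its top cube and temporarily becomes single.
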(event `self.ReceiveBeginPlay`
  (bind _powerupmeshtop (`self.PowerUpMeshTop`))
  ;[1 1 1] Init
  (set `self.m_active?` true)
  (`|ExecutionSequence`
    (:`then_0`
      (`SceneComponent.SetVisibility` (`self.PowerUpMeshBottom`) true true)
      (if (`self.m_doubleBlock`)
        (`SceneComponent.SetVisibility` _powerupmeshtop true true)
        (else
          (`SceneComponent.SetVisibility` _powerupmeshtop false true))))
    (:`then_1`
      (bind (_direction _rotation) (`Timeline|SpiningCube` :!via `PlayFromStart`)
        (:`Update`
          (`SceneComponent.K2_SetRelativeRotation` (`self.PowerUpMeshBottom`) (`KismetMathLibrary.MakeRotator` _rotation _rotation _rotation) false false)
          (`SceneComponent.K2_SetRelativeRotation` (`self.PowerUpMeshTop`) (`KismetMathLibrary.MakeRotator` _rotation _rotation _rotation) false false))))
    (:`then_2`
      (set `self.m_spawnedAsDouble` (`self.m_doubleBlock`)))
    (:`then_3`
      (bind _outactors (`GameplayStatics.GetAllActorsOfClass` "/Game/KartController/BP_KartController.BP_KartController_C"))
      (set `self.As BP Kart Controller` (`|GetArrayItem` _outactors))
      (set `self.m_defaultTransform` (`self.GetTransform`)))))

(event `self.HitBox.OnComponentBeginOverlap`
  (params (OverlappedComponent :type "PrimitiveComponent Object Reference") (OtherActor :type "Actor Object Reference") (OtherComp :type "PrimitiveComponent Object Reference") (OtherBodyIndex :type Integer) (bFromSweep :type Boolean) (SweepResult :type "HitResult Structure (by ref)"))
  (bind _as_bp_kart_controller (`self.As BP Kart Controller`))
  (bind (_m_defaulttransform_location _m_defaulttransform_rotation _m_defaulttransform_scale) (`KismetMathLibrary.BreakTransform` (`self.m_defaultTransform`)))
  (bind _m_enumarr (`self.M_EnumArr`))
  (bind (_m_defaulttransform_location_2 _m_defaulttransform_rotation_2 _m_defaulttransform_scale_2) (`KismetMathLibrary.BreakTransform` (`self.m_defaultTransform`)))
  (bind _as_bp_kart_controller_2 (`self.As BP Kart Controller`))
  (bind _output (`|GetArrayItem` _m_enumarr (`KismetMathLibrary.RandomIntegerInRange` 1 (`KismetArrayLibrary.Array_Length` _m_enumarr))))
  ;[1 1 1] Begin Overlap
  (if (`self.m_active?`)
    (bind _asbp_kart_controller (cast `/Game/KartController/BP_KartController` OtherActor))
    (if (and (`/Game/KartController/BP_KartController.m_hasPrimaryPowerUp` _asbp_kart_controller) (`/Game/KartController/BP_KartController.m_hasSecondaryPowerUp` _asbp_kart_controller))
      _
      (elif (`self.m_doubleBlock`)
        (if (`/Game/KartController/BP_KartController.m_hasPrimaryPowerUp` (`self.As BP Kart Controller`))
          (set `self.m_doubleBlock` false)
          (`|ExecutionSequence`
            (:`then_0`
              (`KismetSystemLibrary.Delay` (`self.m_deactivatedDuration`))
              (if (not (`self.m_doubleBlock`))
                (set `self.m_doubleBlock` true)
                (bind (_direction _scalemultiplier) (`Timeline|Timeline_0` :!via `ReverseFromEnd`)
                  (:`Update`
                    (`SceneComponent.SetRelativeScale3D` (`self.PowerUpMeshTop`) (* _m_defaulttransform_scale _scalemultiplier))))))
            (:`then_1`
              (bind (_direction_2 _scalemultiplier_2) (`Timeline|PickupScaleTimeline2` :!via `PlayFromStart`)
                (:`Update`
                  (`SceneComponent.SetRelativeScale3D` (`self.PowerUpMeshTop`) (* _m_defaulttransform_scale_2 _scalemultiplier_2)))
                (:`Finished`
                  (set `/Game/KartController/BP_KartController.m_hasSecondaryPowerUp` true (`self.As BP Kart Controller`))
                  (if (`/Game/KartController/BP_KartController.m_hasPrimaryPowerUp` (`self.As BP Kart Controller`)) :!label _label
                    (if (not (`/Game/KartController/BP_KartController.m_hasSecondaryPowerUp` (`self.As BP Kart Controller`)))
                      (bind _output_get (set `/Game/KartController/BP_KartController.m_secondaryPowerUpEnum` _output _as_bp_kart_controller_2))
                      (`KismetSystemLibrary.PrintString` (`|GetEnumeratorNameAsString` _output_get))
                      (set `/Game/KartController/BP_KartController.m_hasSecondaryPowerUp` true _as_bp_kart_controller)
                      (`/Game/UI/UI_Widgets/HUD/UI_Pickup.DisplayChosenPUSecondary` (`/Game/UI/UI_Widgets/HUD/UI_HUD.UI_Pickup` (`/Game/KartController/BP_KartController.m_UI_HUD` _as_bp_kart_controller)) (`KismetMathLibrary.Conv_ByteToInt` _output_get)))
                    (else
                      (bind _output_get_2 (set `/Game/KartController/BP_KartController.m_primaryPowerUpEnum` _output _as_bp_kart_controller_2))
                      (`KismetSystemLibrary.PrintString` (`|GetEnumeratorNameAsString` _output_get_2))
                      (set `/Game/KartController/BP_KartController.m_hasPrimaryPowerUp` true _as_bp_kart_controller)
                      (`/Game/KartController/BP_KartController.SpawnPrimaryPowerUp` (`self.As BP Kart Controller`) false)))))))
          (else
            (for _ (range 2)
              (goto _label))
            (`self.Deactivate`)
            (`KismetSystemLibrary.Delay` (`self.m_deactivatedDuration`))
            (`self.Activate`)
            (`KismetSystemLibrary.PrintString` "Hello")))
        (else
          (`|ExecutionSequence`
            (:`then_0`
              (goto _label))
            (:`then_1`
              (`self.Deactivate`)
              (`KismetSystemLibrary.Delay` (`self.m_deactivatedDuration`))
              (`self.Activate`))))))))

(event `Activate`
  (bind (_m_defaulttransform_location _m_defaulttransform_rotation _m_defaulttransform_scale) (`KismetMathLibrary.BreakTransform` (`self.m_defaultTransform`)))
  ;[1 1 1] Activation and Deactivation
  (`KismetSystemLibrary.PrintString` "ACTIVATE" true true (struct :`R` 0.133017 :`G` 1.0 :`A` 1.0))
  (`PrimitiveComponent.SetCollisionEnabled` (`self.HitBox`) "QueryOnly")
  (set `self.m_active?` true)
  (bind (_direction _scalemultiplier) (`Timeline|PickupScaleTimeline` :!via `ReverseFromEnd` :!label _label_2)
    (:`Update`
      (`self.SetActorScale3D` (* _m_defaulttransform_scale _scalemultiplier)))))

(event `Deactivate`
  ;[1 1 1] Activation and Deactivation
  (`KismetSystemLibrary.PrintString` "DEACTIVATE" true true (struct :`R` 1.0 :`G` 0.079836 :`A` 1.0))
  (`PrimitiveComponent.SetCollisionEnabled` (`self.HitBox`) "NoCollision")
  (set `self.m_active?` false)
  (goto _label_2 :!via `PlayFromStart`))

(fn `UserConstructionScript`)