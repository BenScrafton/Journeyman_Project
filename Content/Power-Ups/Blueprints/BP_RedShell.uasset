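; BP_RedShell is a red shell power-up actor that travels along the spline held by its MSpline reference.
; On BeginPlay it derives StartTime from a zero distance, scales Duration by it (making both zero), then calls MoveObject.
; MoveObject sets the ShellMover timeline's play rate to the inverse of Duration and plays it from StartTime.
; Each update maps Alpha to distance along the spline, setting world location and rotation.
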(event `self.ReceiveBeginPlay`
  (bind _output_get (set `self.Start time` (/ 0.0 (`SplineComponent.GetSplineLength` (`/Game/Maps/AI/Spline.Spline` (`self.m_spline`))))))
  (set `self.duration` (* _output_get (`self.duration`)))
  (`self.MoveObject`))

(event `MoveObject`
  (bind _shell_mover (`self.Shell Mover`))
  (bind _spline (`/Game/Maps/AI/Spline.Spline` (`self.m_spline`)))
  (bind _returnvalue (`KismetMathLibrary.Lerp` 0.0 (`SplineComponent.GetSplineLength` _spline) (`self.Alpha`)))
  (`TimelineComponent.SetPlayRate` _shell_mover (/ 1.0 (`self.duration`)))
  (`TimelineComponent.SetNewTime` _shell_mover (`self.Start time`))
  (bind (_direction _alpha) (`Timeline|Shell Mover`)
    (:`Update`
      (set `self.Alpha` _alpha)
      (`self.K2_SetActorLocationAndRotation` (`SplineComponent.GetLocationAtDistanceAlongSpline` _spline _returnvalue "World") (`SplineComponent.GetRotationAtDistanceAlongSpline` _spline _returnvalue "World")))))

(fn `UserConstructionScript`)