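; Coin pickup that rewards an overlapping BP_KartController with coin value and is meant to raise its max velocity.
; On overlap it calls the kart's CoinPickup, then picks a sound by collected count for rising feedback.
; Counts 1 to 11 also spawn an explosion and destroy the coin.
; The speed increase follows a short Delay on the same actor, so that destruction preempts it.
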(event `self.ReceiveBeginPlay`
  ;[1 0 0] EVENT BEGINPLAY
  ;[1 1 1] Change Coin Scale & Coin Value
  (`SceneComponent.SetRelativeScale3D` (`self.MESH_Coin`) (`KismetMathLibrary.MakeVector` (`self.m_Coin Mesh XScale`) (`self.m_Coin Mesh YScale`)))
  (bind _output_get (set `self.m_CoinValueModifier` (`self.m_CoinValueModifier`))))

(event `self.SphereCollision.OnComponentBeginOverlap`
  (params (OverlappedComponent :type "PrimitiveComponent Object Reference") (OtherActor :type "Actor Object Reference") (OtherComp :type "PrimitiveComponent Object Reference") (OtherBodyIndex :type Integer) (bFromSweep :type Boolean) (SweepResult :type "HitResult Structure (by ref)"))
  (bind _kartref (`self.KartREF`))
  (bind _returnvalue (`SceneComponent.K2_GetComponentLocation` (`self.MESH_Coin`)))
  ;[1 0 0] EVENT BEGIN OVERLAP
  ;[1 1 1] Checks for player
  (bind _asbp_kart_controller (cast `/Game/KartController/BP_KartController` OtherActor))
  (set `self.KartREF` _asbp_kart_controller)
  ;[0.2916 0.3628 1] Adds speed modifier to max speed after 3 seconds
  ;;[1 1 1] KartBP Function
  (`/Game/KartController/BP_KartController.CoinPickup` _asbp_kart_controller (stale `self.ReceiveBeginPlay` _output_get))
  (`|ExecutionSequence`
    (:`then_0`
      ;[1 1 1] Checks how many coins have been collected to give different pitches for each collected
      (switch `int` (`/Game/KartController/BP_KartController.m_CoinsCollected` _kartref)
        (:`1`
          (`GameplayStatics.PlaySoundAtLocation` "/Game/Audio/CoinPickup/S_CoinPickupSound01.S_CoinPickupSound01" _returnvalue (struct) 1.0 1.0 0.0 null null null))
        (:`2`
          (`GameplayStatics.PlaySoundAtLocation` "/Game/Audio/CoinPickup/PitchAlternates/S_CoinPickupSound02.S_CoinPickupSound02" _returnvalue (struct) 1.0 1.0 0.0 null null null))
        (:`3`
          (`GameplayStatics.PlaySoundAtLocation` "/Game/Audio/CoinPickup/PitchAlternates/S_CoinPickupSound03.S_CoinPickupSound03" _returnvalue (struct) 1.0 1.0 0.0 null null null))
        (:`4`
          (`GameplayStatics.PlaySoundAtLocation` "/Game/Audio/CoinPickup/PitchAlternates/S_CoinPickupSound04.S_CoinPickupSound04" _returnvalue (struct) 1.0 1.0 0.0 null null null))
        (:`5`
          (`GameplayStatics.PlaySoundAtLocation` "/Game/Audio/CoinPickup/PitchAlternates/S_CoinPickupSound05.S_CoinPickupSound05" _returnvalue (struct) 1.0 1.0 0.0 null null null))
        (:`6`
          (`GameplayStatics.PlaySoundAtLocation` "/Game/Audio/CoinPickup/PitchAlternates/S_CoinPickupSound06.S_CoinPickupSound06" _returnvalue (struct) 1.0 1.0 0.0 null null null))
        (:`7`
          (`GameplayStatics.PlaySoundAtLocation` "/Game/Audio/CoinPickup/PitchAlternates/S_CoinPickupSound07.S_CoinPickupSound07" _returnvalue (struct) 1.0 1.0 0.0 null null null))
        (:`8`
          (`GameplayStatics.PlaySoundAtLocation` "/Game/Audio/CoinPickup/PitchAlternates/S_CoinPickupSound08.S_CoinPickupSound08" _returnvalue (struct) 1.0 1.0 0.0 null null null))
        (:`9`
          (`GameplayStatics.PlaySoundAtLocation` "/Game/Audio/CoinPickup/PitchAlternates/S_CoinPickupSound09.S_CoinPickupSound09" _returnvalue (struct) 1.0 1.0 0.0 null null null))
        (:`10`
          (`GameplayStatics.PlaySoundAtLocation` "/Game/Audio/CoinPickup/PitchAlternates/S_CoinPickupSound10.S_CoinPickupSound10" _returnvalue (struct) 1.0 1.0 0.0 null null null))
        (:`11`
          (`GameplayStatics.PlaySoundAtLocation` "/Game/Audio/CoinPickup/PitchAlternates/S_CoinPickupSound11.S_CoinPickupSound11" _returnvalue (struct) 1.0 1.0 0.0 null null null)))
      ;[1 1 1] Spawns a particle effect at the coin location and removes the BP
      (`GameplayStatics.SpawnEmitterAtLocation` "/Game/StarterContent/Particles/P_Explosion.P_Explosion" _returnvalue (struct) (1.5 1.5 1.5))
      (`self.K2_DestroyActor`))
    (:`then_1`
      (`KismetSystemLibrary.Delay` 0.2)
      (set `/Game/KartController/BP_KartController.m_maxVelocity` (+ (`/Game/KartController/BP_KartController.m_maxVelocity` _asbp_kart_controller) (`self.m_KartMaxSpeedModifier`)) _kartref))))

(fn `UserConstructionScript`)