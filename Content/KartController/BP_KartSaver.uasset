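; BP_KartSaver rescues a kart by carrying it back to its last checkpoint.
; RescueKart looks up that checkpoint in Mario_GameMode's list using the kart's MLastCheckpoint, zeroes its velocity and flags it as rescuing.
; Tick lerps the kart body from its original position to the checkpoint, then clears both flags.
; The checkpoint array gathered at BeginPlay is unused, and nearest-distance search fragments never run.
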(event `RescueKart`
  (bind _m_kart (`self.m_kart`))
  (bind _asmario_game_mode (cast `/Game/Mario_GameMode` (`GameplayStatics.GetGameMode`)))
  (set `self.m_nearestCheckpoint` (`|GetArrayItem` (`/Game/Mario_GameMode.Checkponts` _asmario_game_mode) (- (`/Game/KartController/BP_KartController.m_lastCheckpoint` (`self.m_kart`)) 1)))
  (set `/Game/KartController/BP_KartController.m_rescuing` true (`self.m_kart`))
  (set `self.m_rescuing` true)
  (set `self.m_origKartPos` (`SceneComponent.K2_GetComponentLocation` (`/Game/KartController/BP_KartController.Body` _m_kart)))
  (set `/Game/KartController/BP_KartController.m_curVelocity` 0.0 _m_kart))

(event `self.ReceiveBeginPlay`
  (bind _outactors (`GameplayStatics.GetAllActorsOfClass` "/Game/Checkpoint/Checkpoint_BP.Checkpoint_BP_C"))
  (set `self.m_checkpoints` _outactors))

(event `InitKart`
  (params (NewParam :type "/Game/KartController/BP_KartController Object Reference"))
  (set `self.m_kart` NewParam))

(event `self.ReceiveTick`
  (params (DeltaSeconds :type "Float (single-precision)"))
  (if (`self.m_rescuing`)
    (bind _output_get (set `self.m_alpha` (+ (* (`GameplayStatics.GetWorldDeltaSeconds`) (`self.m_rescueSpeed`)) (`self.m_alpha`))))
    (`SceneComponent.K2_SetWorldLocation` (`/Game/KartController/BP_KartController.Body` (`self.m_kart`)) (`KismetMathLibrary.VLerp` (`self.m_origKartPos`) (`SceneComponent.K2_GetComponentLocation` (`/Game/Checkpoint/Checkpoint_BP.DefaultSceneRoot` (`self.m_nearestCheckpoint`))) _output_get) false false)
    (if (>= (`self.m_alpha`) 1.0)
      (set `self.m_rescuing` false)
      (set `/Game/KartController/BP_KartController.m_rescuing` false (`self.m_kart`))
      (set `self.m_alpha` 0.0))))