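; Player kart controller with hand-written arcade physics, hop-and-drift steering and a two-slot powerup inventory that currently always fires a green shell.
; BeginPlay loads tuning from BPKartParameters; each Tick applies gravity, orientation and movement by directly offsetting and rotating components.
; Downward line traces handle grounding and slope pitch/roll, easing the kart level when airborne.
; Drifting offsets travel direction from body facing after a short delay; AdjustCamera is never called.
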(event `InputAction|Use Powerup`
  (params (Key :type "Key Structure"))
  (:`Pressed`
    (`self.PowerupUse`)))

(event `self.ReceiveTick`
  (params (DeltaSeconds :type "Float (single-precision)"))
  (`self.ApplyGravity`)
  (`self.OrientKart`)
  (`self.ApplyKartMovement`))

(event `self.Body.OnComponentHit`
  (params (HitComponent :type "PrimitiveComponent Object Reference") (OtherActor :type "Actor Object Reference") (OtherComp :type "PrimitiveComponent Object Reference") (NormalImpulse :type "Vector Structure") (Hit :type "HitResult Structure (by ref)"))
  (`KismetSystemLibrary.PrintString` "Hello"))

(event `self.ReceiveBeginPlay`
  (bind _returnvalue_x (`KismetMathLibrary.BreakVector` (`SceneComponent.K2_GetComponentLocation` (`self.F_TraceStart`))))
  (bind _returnvalue_x_2 (`KismetMathLibrary.BreakVector` (`SceneComponent.K2_GetComponentLocation` (`self.B_TraceStart`))))
  (bind (_relativelocation_x _relativelocation_y) (`KismetMathLibrary.BreakVector` (`SceneComponent.RelativeLocation` (`self.FR_TraceStart`))))
  (bind (_relativelocation_x_2 _relativelocation_y_2) (`KismetMathLibrary.BreakVector` (`SceneComponent.RelativeLocation` (`self.FL_TraceStart`))))
  (bind _returnvalue (`KismetMathLibrary.Abs` (- _relativelocation_y_2 _relativelocation_y)))
  ;[1 1 1] Initialise
  (`self.InitialiseKartParameters`)
  (set `self.m_curDirection` (`SceneComponent.GetForwardVector` (`self.Body`)))
  (set `self.m_xKartLength` (`KismetMathLibrary.Abs` (- _returnvalue_x _returnvalue_x_2)))
  (set `self.m_yKartWidth` _returnvalue)
  (`KismetSystemLibrary.PrintString` (`KismetStringLibrary.Conv_DoubleToString` _returnvalue) true true (struct :`R` 1.0 :`B` 0.065503 :`A` 1.0)))

(event `InputAction|Drift`
  (params (Key :type "Key Structure"))
  (:`Pressed`
    ;[1 1 1] Start Drift
    (`self.Jump`)
    (if (!= (`self.GetInputAxisValue`) 0.0)
      (`self.InitialiseDriftParameters`)
      (set `self.m_isDrifting` true)))
  (:`Released`
    ;[1 1 1] End Drift
    (set `self.m_isDrifting` false)))

(fn `Accelerate`
  (bind _returnvalue (+ (`self.m_curVelocity`) (* (`GameplayStatics.GetWorldDeltaSeconds`) (`self.m_acceleration`) (`self.GetInputAxisValue`))))
  ;[1 1 1] accelerate
  ;;[1 1 1] check if the velocity is less than the max
  (if (> (`self.m_maxVelocity`) _returnvalue)
    ;;[1 1 1] set appropriate velocity
    (set `self.m_curVelocity` _returnvalue)
    (else
      (set `self.m_curVelocity` (`self.m_maxVelocity`)))))

(fn `AdjustCamera`
  (if (== (`self.m_curDirection`) (`SceneComponent.GetForwardVector` (`self.CameraDirVectorArm`)) :`ErrorTolerance` 0.01)
    _
    (elif (`self.m_isDrifting`)
      (`SceneComponent.K2_AddWorldRotation` (`self.SpringArm`) (`KismetMathLibrary.MakeRotator` 0.0 0.0 (* (`GameplayStatics.GetWorldDeltaSeconds`) (`self.m_cameraRotateSpeed`) (`self.m_previousDriftDir`) -1.0)) false false)
      (else
        (`SceneComponent.K2_AddWorldRotation` (`self.SpringArm`) (`KismetMathLibrary.MakeRotator` 0.0 0.0 (* (`GameplayStatics.GetWorldDeltaSeconds`) (`self.m_cameraRotateSpeed`) (`self.m_previousDriftDir`))) false false)))))

(fn `ApplyGravity`
  (bind _m_groundchecktracelength (`self.m_groundCheckTraceLength`))
  (bind _returnvalue (`self.CheckGrounded`))
  (if _returnvalue
    (set `self.m_fallingSpeed` 0.0)
    (bind _disttoground (`self.GetDistToGround`))
    (if (< _disttoground _m_groundchecktracelength)
      (`SceneComponent.K2_AddWorldOffset` (`self.Body`) (* (`SceneComponent.GetUpVector` (`self.Body`)) (- _m_groundchecktracelength _disttoground)) true false))
    (else
      (set `self.m_fallingSpeed` (+ (`self.m_fallingSpeed`) (* (`GameplayStatics.GetWorldDeltaSeconds`) (`self.m_gravityStrength`))))
      (bind _disttoground_2 (`self.GetDistToGround`))
      (if (< _disttoground_2 (`self.m_fallingSpeed`))
        (`SceneComponent.K2_AddWorldOffset` (`self.Body`) (* (`SceneComponent.GetUpVector` (`self.Body`)) (* -1 (- _disttoground_2 (`self.m_groundCheckTraceLength`)))) true false)
        (else
          (`SceneComponent.K2_AddWorldOffset` (`self.Body`) (`KismetMathLibrary.MakeVector` 0.0 0.0 (* -1 (`self.m_fallingSpeed`))) true false))))))

(fn `ApplyKartMovement`
  (`self.CalculateCurVelocity`)
  (if (`self.m_isDrifting`)
    (`self.Drift`)
    (bind _returnvalue (`self.CheckGrounded`))
    (if (and _returnvalue (> (`self.m_driftTime`) 0.5))
      (`self.SetDriftVector`))
    (else
      (set `self.m_driftTime` 0.0)
      (`self.DefaultSteer`)))
  (`self.Move`))

(fn `CalculateCurVelocity`
  ;[1 1 1] check acceleration direction (forwards/backwards)
  (`self.SetIsAccelerating`)
  (if (`self.m_isAccelerating`)
    (bind _returnvalue (`self.CheckGrounded`))
    (if _returnvalue
      (`self.Accelerate`))
    (else
      (bind _returnvalue_2 (`self.CheckGrounded`))
      (if _returnvalue_2
        (`self.Decelerate`)))))

(fn `CalculateTargetPitch`
  (returns (pitch :type "Float (double-precision)"))
  (locals (frontDist :type "Float (double-precision)") (backDist :type "Float (double-precision)") (zValue :type "Float (double-precision)") (targetPitch :type "Float (double-precision)") (surfaceNorm :type "Vector Structure") (temp :type "Float (double-precision)"))
  (bind _returnvalue (`SceneComponent.K2_GetComponentLocation` (`self.F_TraceStart`)))
  (bind _returnvalue_2 (`SceneComponent.K2_GetComponentLocation` (`self.B_TraceStart`)))
  (bind (_outhit _returnvalue_3) (`KismetSystemLibrary.LineTraceSingle` :`Start` _returnvalue :`End` (+ (* (`SceneComponent.GetUpVector` (`self.Body`)) (* -1 (`self.m_floorTraceLength`))) _returnvalue) :`TraceChannel` "TraceTypeQuery1" :`DrawDebugType` "ForOneFrame"))
  (if _returnvalue_3
    (bind _output_get (set `local.frontDist` (`.Distance` (`GameplayStatics.BreakHitResult` _outhit))))
    (bind (_outhit_2 _returnvalue_4) (`KismetSystemLibrary.LineTraceSingle` :`Start` _returnvalue_2 :`End` (+ (* (`SceneComponent.GetUpVector` (`self.Body`)) (* -1 (`self.m_floorTraceLength`))) _returnvalue_2) :`TraceChannel` "TraceTypeQuery1" :`DrawDebugType` "ForOneFrame"))
    (if _returnvalue_4
      (set `local.backDist` (`.Distance` (`GameplayStatics.BreakHitResult` _outhit_2)))
      (set `local.zValue` (- (`local.backDist`) (`local.frontDist`)))
      (set `local.targetPitch` (`KismetMathLibrary.DegAtan` (/ (`local.zValue`) (`self.m_xKartLength`))))
      (return (`local.targetPitch`))
      (else
        (set `local.targetPitch` 0.0)))
    (else
      (set `local.targetPitch` 0.0))))

(fn `CalculateTargetRoll`
  (returns (roll :type "Float (double-precision)"))
  (locals (leftDist :type "Float (double-precision)") (rightDist :type "Float (double-precision)") (zValue :type "Float (double-precision)") (targetRoll :type "Float (double-precision)"))
  (bind _returnvalue (`SceneComponent.K2_GetComponentLocation` (`self.FL_TraceStart`)))
  (bind _returnvalue_2 (`SceneComponent.K2_GetComponentLocation` (`self.FR_TraceStart`)))
  (bind (_outhit _returnvalue_3) (`KismetSystemLibrary.LineTraceSingle` :`Start` _returnvalue :`End` (+ (* (`SceneComponent.GetUpVector` (`self.Body`)) (* -1 (`self.m_floorTraceLength`))) _returnvalue) :`TraceChannel` "TraceTypeQuery1" :`DrawDebugType` "ForOneFrame"))
  (if _returnvalue_3
    (set `local.leftDist` (`.Distance` (`GameplayStatics.BreakHitResult` _outhit)))
    (bind (_outhit_2 _returnvalue_4) (`KismetSystemLibrary.LineTraceSingle` :`Start` _returnvalue_2 :`End` (+ (* (`SceneComponent.GetUpVector` (`self.Body`)) (* -1 (`self.m_floorTraceLength`))) _returnvalue_2) :`TraceChannel` "TraceTypeQuery1" :`DrawDebugType` "ForOneFrame"))
    (if _returnvalue_4
      (set `local.rightDist` (`.Distance` (`GameplayStatics.BreakHitResult` _outhit_2)))
      (set `local.zValue` (- (`local.rightDist`) (`local.leftDist`)))
      (set `local.targetRoll` (`KismetMathLibrary.DegAtan` (/ (`local.zValue`) (`self.m_yKartWidth`))))
      (return (`local.targetRoll`))
      (else
        (set `local.targetRoll` 0.0)))
    (else
      (set `local.targetRoll` 0.0))))

(fn `CheckGrounded`
  (returns (ReturnValue :type Boolean))
  (bind _returnvalue (`SceneComponent.K2_GetComponentLocation` (`self.Body`)))
  (bind (_outhit _returnvalue_2) (`KismetSystemLibrary.LineTraceSingle` :`Start` _returnvalue :`End` (+ _returnvalue (`KismetMathLibrary.TransformDirection` (`self.GetTransform`) (`KismetMathLibrary.MakeVector` 0.0 0.0 (- (* (`self.m_groundCheckTraceLength`) -1.0) 10.0)))) :`TraceChannel` "TraceTypeQuery1" :`DrawDebugType` "ForOneFrame" :`TraceColor` (struct :`R` 1.0 :`B` 0.660388 :`A` 1.0)))
  (return _returnvalue_2))

(fn `Decelerate`
  (bind _returnvalue (- (`self.m_curVelocity`) (* (`self.m_deceleration`) (`GameplayStatics.GetWorldDeltaSeconds`))))
  (bind _returnvalue_2 (+ (`self.m_curVelocity`) (* (`self.m_deceleration`) (`GameplayStatics.GetWorldDeltaSeconds`))))
  (if (> (`self.m_curVelocity`) 0.0)
    ;[1 1 1] decelerate A
    ;;[1 1 1] check if the new velocity is less than 0
    (if (<= _returnvalue 0.0)
      ;;[1 1 1] set appropriate velocity
      (set `self.m_curVelocity` 0.0)
      (else
        (set `self.m_curVelocity` _returnvalue)))
    (else
      ;[1 1 1] decelerate B
      ;;[1 1 1] check if the new velocity is less than 0
      (if (>= _returnvalue_2 0.0)
        ;;[1 1 1] set appropriate velocity
        (set `self.m_curVelocity` 0.0)
        (else
          (set `self.m_curVelocity` _returnvalue_2))))))

(fn `DefaultSteer`
  (if (!= (`self.m_curVelocity`) 0.0)
    (`SceneComponent.K2_AddLocalRotation` (`self.Body`) (`KismetMathLibrary.MakeRotator` 0.0 0.0 (* (`self.GetInputAxisValue`) (* (`self.m_steerFactor`) (+ (/ (`self.m_curVelocity`) (`self.m_maxVelocity`)) 0.5)))) true false)
    (set `self.m_curDirection` (`SceneComponent.GetForwardVector` (`self.Body`)))))

(fn `Drift`
  (bind _m_previousdriftdir (`self.m_previousDriftDir`))
  (bind (_relativerotation_roll _relativerotation_pitch _relativerotation_yaw) (`KismetMathLibrary.BreakRotator` (`SceneComponent.RelativeRotation` (`self.Body`))))
  (`SceneComponent.K2_SetRelativeRotation` (`self.Body`) (`KismetMathLibrary.MakeRotator` _relativerotation_roll _relativerotation_pitch (+ _relativerotation_yaw (* (`GameplayStatics.GetWorldDeltaSeconds`) (`self.m_driftFactor`) (/ (+ _m_previousdriftdir (`self.GetInputAxisValue`) (* _m_previousdriftdir 0.5)) 2.0) 1.0))) true false)
  (set `self.m_driftTime` (+ (`self.m_driftTime`) (`GameplayStatics.GetWorldDeltaSeconds`))))

(fn `GetDistToGround`
  (returns (distToGround :type "Float (double-precision)"))
  (locals (dist :type "Float (double-precision)"))
  (bind (_outhit _returnvalue) (`KismetSystemLibrary.LineTraceSingle` (`SceneComponent.K2_GetComponentLocation` (`self.Body`)) (+ (`SceneComponent.K2_GetComponentLocation` (`self.Body`)) (* (`SceneComponent.GetUpVector` (`self.Body`)) -2147483648)) "TraceTypeQuery1"))
  (if _returnvalue
    (set `local.dist` (`.Distance` (`GameplayStatics.BreakHitResult` _outhit)))
    (else
      (set `local.dist` 100000000.0)))
  (return (`local.dist`)))

(fn `InitialiseDriftParameters`
  (set `self.m_previousDriftDir` (`self.GetInputAxisValue`))
  (set `self.m_driftStartKartRot` (`SceneComponent.RelativeRotation` (`self.Body`)))
  (set `self.m_driftStartCameraRot` (`SceneComponent.RelativeRotation` (`self.SpringArm`))))

(fn `InitialiseKartParameters`
  (set `self.m_acceleration` (`/Game/KartController/BP_KartParameters.m_acceleration` (`self.BP_KartParameters`)))
  (set `self.m_maxVelocity` (`/Game/KartController/BP_KartParameters.m_maxVelocity` (`self.BP_KartParameters`)))
  (set `self.m_deceleration` (`/Game/KartController/BP_KartParameters.m_deceleration` (`self.BP_KartParameters`)))
  (set `self.m_steerFactor` (`/Game/KartController/BP_KartParameters.m_steerFactor` (`self.BP_KartParameters`)))
  (set `self.m_driftFactor` (`/Game/KartController/BP_KartParameters.m_driftFactor` (`self.BP_KartParameters`)))
  (set `self.m_initalKartDriftAngle` (`/Game/KartController/BP_KartParameters.m_initKartDriftAngle` (`self.BP_KartParameters`)))
  (set `self.m_orientSpeed` (`/Game/KartController/BP_KartParameters.m_orientSpeed` (`self.BP_KartParameters`))))

(fn `Jump`
  (bind _returnvalue (`self.CheckGrounded`))
  (if _returnvalue
    (`SceneComponent.K2_AddLocalOffset` (`self.Body`) (* (`SceneComponent.GetUpVector` (`self.Body`)) 10.0) true false)
    (set `self.m_fallingSpeed` (`self.m_jumpStrength`))))

(fn `Move`
  (`SceneComponent.K2_SetWorldLocation` (`self.Body`) (+ (`SceneComponent.K2_GetComponentLocation` (`self.Body`)) (* (`self.m_curDirection`) (`self.m_curVelocity`))) true false))

(fn `OrientKart`
  (locals (neutralRotateApha :type "Float (double-precision)") (neutralRotateAphaFactor :type "Float (double-precision)" :default 2.0) (neutralising :type Boolean))
  (bind _returnvalue (* 0.1 1.0))
  (bind _neutralrotateapha (`local.neutralRotateApha`))
  (bind (_relativerotation_roll _relativerotation_pitch _relativerotation_yaw) (`KismetMathLibrary.BreakRotator` (`SceneComponent.RelativeRotation` (`self.Body`))))
  (if (`self.neutralisingRot`)
    (set `local.neutralRotateApha` (+ (* (`local.neutralRotateAphaFactor`) (`GameplayStatics.GetWorldDeltaSeconds`)) (`local.neutralRotateApha`)))
    (else
      (set `local.neutralRotateApha` 0.0)))
  (bind (_outhit _returnvalue_2) (`KismetSystemLibrary.LineTraceSingle` :`Start` (`SceneComponent.K2_GetComponentLocation` (`self.C_TraceStart`)) :`End` (+ (`SceneComponent.K2_GetComponentLocation` (`self.C_TraceStart`)) (* (`SceneComponent.GetUpVector` (`self.Body`)) -150.0)) :`TraceChannel` "TraceTypeQuery1" :`DrawDebugType` "ForOneFrame" :`TraceColor` (struct :`R` 0.524927 :`G` 1.0 :`B` 0.70011 :`A` 1.0)))
  (if _returnvalue_2
    (set `self.neutralisingRot` false)
    (else
      (set `self.neutralisingRot` true)
      (`SceneComponent.K2_SetRelativeRotation` (`self.Body`) (`KismetMathLibrary.RLerp` (`SceneComponent.RelativeRotation` (`self.Body`)) (`KismetMathLibrary.MakeRotator` 0.0 0.0 _relativerotation_yaw) _neutralrotateapha) true false)
      (`KismetSystemLibrary.PrintString` (`KismetStringLibrary.Conv_DoubleToString` _neutralrotateapha))))
  (bind _pitch (`self.CalculateTargetPitch`))
  (bind _roll (`self.CalculateTargetRoll`))
  (`self.K2_AddActorLocalRotation` (`KismetMathLibrary.MakeRotator` (* _roll _returnvalue) (* _pitch _returnvalue)) true))

(fn `PowerupUse`
  (if (`self.m_hasPrimaryPowerUp`)
    (`|SpawnActorFromClass` "/Game/Power-Ups/Blueprints/GreenShell_bp.GreenShell_bp_C" (`SceneComponent.K2_GetComponentToWorld` (`self.Arrow`)) "Undefined" "OverrideRootScale" null null)
    (if (`self.m_hasSecondaryPowerUp`)
      (set `self.m_hasSecondaryPowerUp` false)
      (set `self.m_primaryPowerUpEnum` (`self.m_secondaryPowerUpEnum`))
      (set `self.m_secondaryPowerUpEnum` "NewEnumerator0")
      (else
        (set `self.m_hasPrimaryPowerUp` false)
        (set `self.m_primaryPowerUpEnum` "NewEnumerator0")))))

(fn `SetDriftVector`
  (set `self.m_curDirection` (`KismetMathLibrary.RotateAngleAxis` (`SceneComponent.GetForwardVector` (`self.Body`)) (* (`self.m_previousDriftDir`) (`self.m_initalKartDriftAngle`) -1.0) (`SceneComponent.GetUpVector` (`self.Body`)))))

(fn `SetInitDriftRot`
  (params (Alpha :type "Float (double-precision)"))
  (bind (_m_driftstartkartrot_roll _m_driftstartkartrot_pitch _m_driftstartkartrot_yaw) (`KismetMathLibrary.BreakRotator` (`self.m_driftStartKartRot`)))
  (`SceneComponent.K2_SetRelativeRotation` (`self.Body`) (`KismetMathLibrary.RLerp` (`self.m_driftStartKartRot`) (`KismetMathLibrary.MakeRotator` _m_driftstartkartrot_roll _m_driftstartkartrot_pitch (+ _m_driftstartkartrot_yaw (* (`self.m_initalKartDriftAngle`) (`self.m_previousDriftDir`)))) Alpha) false false))

(fn `SetIsAccelerating`
  (bind _returnvalue (== (`self.GetInputAxisValue`) 0.0))
  (if _returnvalue
    _
    (else
      _))
  (set `self.m_isAccelerating` (not _returnvalue)))

(fn `UserConstructionScript`)