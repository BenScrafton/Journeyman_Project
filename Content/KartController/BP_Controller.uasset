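; BP_Controller is the player controller that drives the kart pawn BP_KartController and sets up the player's HUD.
; On BeginPlay it creates UI_HUD, caches the possessed kart and hands the widget to it.
; While active, it copies steering and throttle axes to the kart every tick, and the Drift action starts a drift or flags its end on release.
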(event `self.ReceiveBeginPlay`
  (bind _returnvalue (`|CreateWidget` "/Game/UI/UI_Widgets/HUD/UI_HUD.UI_HUD_C" self))
  (`UserWidget.AddToViewport` _returnvalue 0)
  (bind _asbp_kart_controller (cast `/Game/KartController/BP_KartController` (`self.K2_GetPawn`)))
  (set `self.m_kart` _asbp_kart_controller)
  (set `/Game/KartController/BP_KartController.m_UI_HUD` _returnvalue (`self.m_kart`)))

(event `InputAction|Drift`
  (params (Key :type "Key Structure"))
  (:`Pressed`
    (if (`self.m_isActive`)
      (`/Game/KartController/BP_KartController.StartDrift` (`self.m_kart`))))
  (:`Released`
    (if (`self.m_isActive`)
      (set `/Game/KartController/BP_KartController.m_endDrift` true (`self.m_kart`)))))

(event `self.ReceiveTick`
  (params (DeltaSeconds :type "Float (single-precision)"))
  (if (`self.m_isActive`)
    (set `/Game/KartController/BP_KartController.m_Left/Right` (`self.GetInputAxisValue`) (`self.m_kart`))
    (set `/Game/KartController/BP_KartController.m_Forward/Backward` (`self.GetInputAxisValue`) (`self.m_kart`))))

(event `InputAction|Use Powerup`
  (params (Key :type "Key Structure")))

(fn `UserConstructionScript`)