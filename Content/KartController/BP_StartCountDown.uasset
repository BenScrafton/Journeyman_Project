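; BP_StartCountDown is an actor that runs a timed start for the kart controllers in the level.
; On BeginPlay it gathers all BP_Controller and AI actors into two arrays, then waits out a short fixed delay.
; It then sets MIsActive to true on each BP_Controller but to false on each AI actor, with no countdown display.
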(event `self.ReceiveBeginPlay`
  (bind _outactors (`GameplayStatics.GetAllActorsOfClass` "/Game/KartController/BP_Controller.BP_Controller_C"))
  (set `self.PlayerControllers` _outactors)
  (bind _outactors_2 (`GameplayStatics.GetAllActorsOfClass` "/Game/Maps/AI/AI.AI_C"))
  (set `self.AI Controllers` _outactors_2)
  (`KismetSystemLibrary.Delay` 3.0)
  (for _array_element (`self.PlayerControllers`)
    (set `/Game/KartController/BP_Controller.m_isActive` true _array_element))
  (for _array_element_2 (`self.AI Controllers`)
    (set `/Game/Maps/AI/AI.m_isActive` false _array_element_2)))

(fn `UserConstructionScript`)