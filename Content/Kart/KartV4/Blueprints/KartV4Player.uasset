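; Player-controlled kart that turns input into handbrake, throttle and steering calls, with mouse orbit on the spring arm.
; Steering eases a value to rotate the steering wheel mesh and sets turn-direction flags; Victory and Boost inputs toggle held-state booleans.
; BeginPlay adds a minimap widget, and Tick creates a new leaderboard widget every frame while LapCounter equals six.
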(event `InputAction|HandBrake`
  (params (Key :type "Key Structure"))
  (:`Pressed`
    (`self.Handbrake` true))
  (:`Released`
    (`self.Handbrake` false)))

(event `InputAxisKey|MouseX`
  (params (AxisValue :type "Float (single-precision)"))
  ;[1 1 1] Camera Stuff - Karl
  (`SceneComponent.K2_AddRelativeRotation` (`self.SpringArm`) (`KismetMathLibrary.MakeRotator` 0.0 0.0 AxisValue) false false))

(event `InputAxis|Throttle`
  (params (AxisValue :type "Float (single-precision)"))
  (`self.Throttle` AxisValue))

(event `InputAxisKey|MouseY`
  (params (AxisValue :type "Float (single-precision)"))
  ;[1 1 1] Camera Stuff - Karl
  (`SceneComponent.K2_AddRelativeRotation` (`self.SpringArm`) (`KismetMathLibrary.MakeRotator` 0.0 AxisValue) false false))

(event `self.ReceiveTick`
  (params (DeltaSeconds :type "Float (single-precision)"))
  (`parent.ReceiveTick` DeltaSeconds)
  (if (== (`self.LapCounter`) 6.0)
    (bind _returnvalue (`|CreateWidget` "/Game/HUD/LeaderBoard.LeaderBoard_C"))
    (`UserWidget.AddToViewport` _returnvalue 0)))

(event `self.ReceiveBeginPlay`
  ;[1 1 1] MiniMap - Julia
  (bind _returnvalue (`|CreateWidget` "/Game/HUD/Minimap/Testing_minimap/Minimap_actual.Minimap_actual_C"))
  (`UserWidget.AddToViewport` _returnvalue 0)
  (set `self.SteeringHome` (`SceneComponent.RelativeRotation` (`self.Steering_Wheel`))))

(event `InputAxis|Steering`
  (params (AxisValue :type "Float (single-precision)"))
  ;[1 1 1] Steering input
  (set `self.IsTurningLeft` (< AxisValue 0.0))
  (set `self.IsTurningRight` (> AxisValue 0.0))
  (set `self.IsNotTurning` (== AxisValue 0.0))
  (set `self.SteeringAmount` (`KismetMathLibrary.FInterpTo` (`self.SteeringAmount`) (* AxisValue 50.0) (`GameplayStatics.GetWorldDeltaSeconds`) 5.0))
  (`self.Steering` AxisValue)
  (`SceneComponent.K2_SetRelativeRotation` (`self.Steering_Wheel`) (`KismetMathLibrary.MakeRotator` (+ (.roll (`self.SteeringHome`)) (* (`self.SteeringAmount`) 1.0)) (.pitch (`self.SteeringHome`)) (.yaw (`self.SteeringHome`))) false false))

(event `InputAction|Victory`
  (params (Key :type "Key Structure"))
  (:`Pressed`
    (set `self.IsVictory` true))
  (:`Released`
    (set `self.IsVictory` false)))

(event `InputAction|Boost`
  (params (Key :type "Key Structure"))
  (:`Pressed`
    (set `self.IsBoosting` true))
  (:`Released`
    (set `self.IsBoosting` false)))

(fn `UserConstructionScript`
  (`parent.UserConstructionScript`))